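; BP_Altar is an interactable altar that a pawn lights up once, offering an "[E]Iluminar" prompt.
; OnInteract sets an active flag, plays an activation sound at the rune and creates a dynamic material instance.
; A timeline ramps the rune's emission, then a loop reveals five point lights.
; The Delay inside that loop does not hold back iteration, so the lights appear together rather than staggered.
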(event `self.ReceiveBeginPlay`)

(event `self.OnInteract`
  (params (InteractorPawn :type "Pawn Object Reference"))
  (bind _baserune (`self.BaseRune`))
  ; Consider transferring this to c++
  (if (not (`self.IsActive`))
    (`KismetSystemLibrary.PrintString` (`KismetSystemLibrary.GetDisplayName` InteractorPawn))
    (`GameplayStatics.PlaySoundAtLocation` (`self.ActivationSound`) (`SceneComponent.K2_GetComponentLocation` (`self.BaseRune`)) (struct) 1.0 1.0 0.0 null null null null)
    (set `self.IsActive` true)
    (bind _returnvalue (`PrimitiveComponent.CreateDynamicMaterialInstance` _baserune 0 (`PrimitiveComponent.GetMaterial` _baserune 0) "None"))
    (bind (_direction _emissiontrack) (`Timeline|TL_MaterialEmission`)
      (:`Update`
        (`MaterialInstanceDynamic.SetScalarParameterValue` _returnvalue "Emission Strength" (* _emissiontrack 15.0)))
      (:`Finished`
        (for _array_element (`|MakeArray` (`self.PointLight`) (`self.PointLight1`) (`self.PointLight2`) (`self.PointLight3`) (`self.PointLight4`))
          (`SceneComponent.SetVisibility` _array_element true false)
          (`KismetSystemLibrary.Delay` 3.0))))))

(fn `GetInteractionPromptText`
  (returns (ReturnValue :type String))
  (return "[E]Iluminar"))

(fn `UserConstructionScript`)