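; BP_Altar is a one-shot interactable altar that lights up when activated.
; Interacting locks further use, plays the pawn's interact animation and triggers a sound at the rune.
; A timeline ramps emission on the rune's dynamic material, then a delayed loop reveals five point lights one at a time.
; It exposes interactable state and prompt text to the interaction system; the rune hover timeline is unconnected.
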(event `self.ReceiveBeginPlay`
  (set `self.PointLights` (`|MakeArray` (`self.PointLight`) (`self.PointLight1`) (`self.PointLight2`) (`self.PointLight3`) (`self.PointLight4`))))

(event `self.OnInteract`
  (params (InteractorPawn :type "Pawn Object Reference"))
  (bind _baserune (`self.BaseRune`))
  (if (`self.IsInteractable`)
    (`|ExecutionSequence`
      (:`then_0`
        (set `self.IsInteractable` false)
        (message `IPlayerInteractions.PlayInteractAnimation` InteractorPawn))
      (:`then_1`
        (`GameplayStatics.PlaySoundAtLocation` (`self.ActivationSound`) (`SceneComponent.K2_GetComponentLocation` (`self.BaseRune`)) (struct) 1.0 1.0 0.0 null null null null))
      (:`then_2`
        (bind _returnvalue (`PrimitiveComponent.CreateDynamicMaterialInstance` _baserune 0 (`PrimitiveComponent.GetMaterial` _baserune 0) "None"))
        (bind (_direction _emissiontrack) (`Timeline|TL_MaterialEmission`)
          (:`Update`
            (`MaterialInstanceDynamic.SetScalarParameterValue` _returnvalue "Emission Strength" (* _emissiontrack 15.0)))
          (:`Finished`
            (bind _array_element (`/Game/GeneralBlueprints/BML_GeneralMacros.ForEachLoopWithDelay` (`self.PointLights`) 0.7)
              (:`LoopBody`
                (`SceneComponent.SetVisibility` _array_element true false)))))))))

(event `self.OnInteractionStop`
  (params (InteractorPawn :type "Pawn Object Reference"))
  (message `IPlayerInteractions.StopLoopingAnimation` InteractorPawn))

(fn `GetInteractableState`
  (returns (ReturnValue :type Boolean))
  (return (`self.IsInteractable`)))

(fn `GetInteractionPromptText`
  (returns (ReturnValue :type String))
  (return (`self.PromptText`)))

(fn `UserConstructionScript`)